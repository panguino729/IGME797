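; BP_DoorBoton is a door actor that swings open or closed when E is pressed near it.
; Overlapping CollitionBox enables input from player controller 0 and prints a prompt, and leaving disables input, with no check on the overlapping actor.
; A FlipFlop on E alternately plays and reverses a timeline, whose Open value scaled by Rotacion drives SMDoor's relative yaw.
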(event `self.CollitionBox.OnComponentBeginOverlap`
  (params (OverlappedComponent :type "PrimitiveComponent Object Reference") (OtherActor :type "Actor Object Reference") (OtherComp :type "PrimitiveComponent Object Reference") (OtherBodyIndex :type Integer) (bFromSweep :type Boolean) (SweepResult :type "HitResult Structure (by ref)"))
  ;[1 1 1 1 30] This will call Of the collition box to see if the character is on it.
  (`self.EnableInput` (`GameplayStatics.GetPlayerController` 0))
  (`KismetSystemLibrary.PrintString` "Press E"))

(event `self.CollitionBox.OnComponentEndOverlap`
  (params (OverlappedComponent :type "PrimitiveComponent Object Reference") (OtherActor :type "Actor Object Reference") (OtherComp :type "PrimitiveComponent Object Reference") (OtherBodyIndex :type Integer))
  ;[1 1 1 1 30] This will call Of the collition box to see if the character is on it.
  (`self.DisableInput` (`GameplayStatics.GetPlayerController` 0)))

(event `Key|E`
  (params (Key :type "Key Structure"))
  ;[1 1 1 1 30] Press botton
  (:`Pressed`
    (`/Engine/EditorBlueprintResources/StandardMacros.FlipFlop`
      (:`A`
        (bind (_direction _open) (`Timeline|Timeline_1` :!label _label)
          (:`Update`
            (`SceneComponent.K2_SetRelativeRotation` (`self.SM_Door`) (`KismetMathLibrary.MakeRotator` 0.0 0.0 (* _open (`self.Rotacion `))) false false))))
      (:`B`
        (goto _label :!via `Reverse`)))))

(fn `UserConstructionScript`)