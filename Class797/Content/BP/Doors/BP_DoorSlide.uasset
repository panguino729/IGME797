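; BP_DoorSlide is an automatic sliding door built from left and right stacks of seven horizontal segments.
; Box overlap plays the DoorL timeline and end overlap reverses it, with no filter on the overlapping actor.
; The MoveL and MoveR tracks drive each segment's relative X at fixed Y and Z.
; Cumulatively nested Lerps use the track value as Alpha, scaling travel down segment by segment up each stack for a stepped slide.
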(event `self.Box.OnComponentBeginOverlap`
  (params (OverlappedComponent :type "PrimitiveComponent Object Reference") (OtherActor :type "Actor Object Reference") (OtherComp :type "PrimitiveComponent Object Reference") (OtherBodyIndex :type Integer) (bFromSweep :type Boolean) (SweepResult :type "HitResult Structure (by ref)"))
  (bind (_direction _movel _mover) (`Timeline|DoorL` :!label _label)
    (:`Update`
      (`SceneComponent.K2_SetRelativeLocation` (`self.SM_SlideDoorL`) (`KismetMathLibrary.MakeVector` _movel -20.0 30.0) false false)
      (bind _returnvalue (`KismetMathLibrary.Lerp` 0.01 0.9 _movel))
      (`SceneComponent.K2_SetRelativeLocation` (`self.SM_SlideDoorL2`) (`KismetMathLibrary.MakeVector` _returnvalue -20.0 65.0) false false)
      (bind _returnvalue_2 (`KismetMathLibrary.Lerp` 0.01 0.93 _returnvalue))
      (`SceneComponent.K2_SetRelativeLocation` (`self.SM_SlideDoorL4`) (`KismetMathLibrary.MakeVector` _returnvalue_2 -20.0 100.0) false false)
      (bind _returnvalue_3 (`KismetMathLibrary.Lerp` 0.01 0.95 _returnvalue_2))
      (`SceneComponent.K2_SetRelativeLocation` (`self.SM_SlideDoorL7`) (`KismetMathLibrary.MakeVector` _returnvalue_3 -20.0 135.0) false false)
      (bind _returnvalue_4 (`KismetMathLibrary.Lerp` 0.01 0.96 _returnvalue_3))
      (`SceneComponent.K2_SetRelativeLocation` (`self.SM_SlideDoorL9`) (`KismetMathLibrary.MakeVector` _returnvalue_4 -20.0 170.0) false false)
      (bind _returnvalue_5 (`KismetMathLibrary.Lerp` 0.01 0.97 _returnvalue_4))
      (`SceneComponent.K2_SetRelativeLocation` (`self.SM_SlideDoorL11`) (`KismetMathLibrary.MakeVector` _returnvalue_5 -20.0 205.0) false false)
      (`SceneComponent.K2_SetRelativeLocation` (`self.SM_SlideDoorL13`) (`KismetMathLibrary.MakeVector` (`KismetMathLibrary.Lerp` 0.01 0.98 _returnvalue_5) -20.0 240.0) false false)
      (bind _returnvalue_6 (`KismetMathLibrary.Lerp` 0.0 0.9 _mover))
      (`SceneComponent.K2_SetRelativeLocation` (`self.SM_SlideDoorR1`) (`KismetMathLibrary.MakeVector` _returnvalue_6 -20.000969 30.0) false false)
      (bind _returnvalue_7 (`KismetMathLibrary.Lerp` 0.1 0.9 _returnvalue_6))
      (`SceneComponent.K2_SetRelativeLocation` (`self.SM_SlideDoorR3`) (`KismetMathLibrary.MakeVector` _returnvalue_7 -20.000969 65.0) false false)
      (bind _returnvalue_8 (`KismetMathLibrary.Lerp` 0.01 0.93 _returnvalue_7))
      (`SceneComponent.K2_SetRelativeLocation` (`self.SM_SlideDoorR5`) (`KismetMathLibrary.MakeVector` _returnvalue_8 -20.000969 100.0) false false)
      (bind _returnvalue_9 (`KismetMathLibrary.Lerp` 0.01 0.95 _returnvalue_8))
      (`SceneComponent.K2_SetRelativeLocation` (`self.SM_SlideDoorR6`) (`KismetMathLibrary.MakeVector` _returnvalue_9 -20.000969 135.0) false false)
      (bind _returnvalue_10 (`KismetMathLibrary.Lerp` 0.01 0.96 _returnvalue_9))
      (`SceneComponent.K2_SetRelativeLocation` (`self.SM_SlideDoorR8`) (`KismetMathLibrary.MakeVector` _returnvalue_10 -20.000969 170.0) false false)
      (bind _returnvalue_11 (`KismetMathLibrary.Lerp` 0.01 0.97 _returnvalue_10))
      (`SceneComponent.K2_SetRelativeLocation` (`self.SM_SlideDoorR10`) (`KismetMathLibrary.MakeVector` _returnvalue_11 -20.000969 205.0) false false)
      (`SceneComponent.K2_SetRelativeLocation` (`self.SM_SlideDoorR12`) (`KismetMathLibrary.MakeVector` (`KismetMathLibrary.Lerp` 0.01 0.98 _returnvalue_11) -20.000969 240.0) false false))))

(event `self.Box.OnComponentEndOverlap`
  (params (OverlappedComponent :type "PrimitiveComponent Object Reference") (OtherActor :type "Actor Object Reference") (OtherComp :type "PrimitiveComponent Object Reference") (OtherBodyIndex :type Integer))
  (goto _label :!via `Reverse`))

(fn `UserConstructionScript`)