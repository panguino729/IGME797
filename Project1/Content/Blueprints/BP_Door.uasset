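; BP_Door is a two-panel sliding metal door that the player opens with E while inside a trigger box.
; Box overlap enables input and opens a gate, so E plays the Door timeline, which slides the two meshes apart along relative X.
; Leaving the box disables input, closes the gate and reverses the timeline.
; SetKeyPress stores a KeyPress value that the event graph does not read.
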(event `self.ReceiveBeginPlay`)

(event `Key|E`
  (params (Key :type "Key Structure"))
  ;[1 1 1] Open door
  (:`Pressed`
    (`/Engine/EditorBlueprintResources/StandardMacros.Gate` true :!label _label
      (:`Exit`
        ;[1 1 1] Animation
        (bind (_direction _float) (`Timeline|Door` :!label _label_2)
          (:`Update`
            (`SceneComponent.K2_SetRelativeLocation` (`self.SM_DoorMetalV1`) (`KismetMathLibrary.MakeVector` (* _float -1.0)) false false)
            (`SceneComponent.K2_SetRelativeLocation` (`self.SM_DoorMetalV2`) (`KismetMathLibrary.MakeVector` _float -30.0) false false)))))))

(event `self.Box.OnComponentBeginOverlap`
  (params (OverlappedComponent :type "PrimitiveComponent Object Reference") (OtherActor :type "Actor Object Reference") (OtherComp :type "PrimitiveComponent Object Reference") (OtherBodyIndex :type Integer) (bFromSweep :type Boolean) (SweepResult :type "HitResult Structure (by ref)"))
  ;[1 1 1] Input
  (`self.EnableInput` (`GameplayStatics.GetPlayerController` 0))
  (goto _label :!via `Open`))

(event `Close`
  ;[1 1 1] Open door
  (goto _label :!via `Close`))

(event `self.Box.OnComponentEndOverlap`
  (params (OverlappedComponent :type "PrimitiveComponent Object Reference") (OtherActor :type "Actor Object Reference") (OtherComp :type "PrimitiveComponent Object Reference") (OtherBodyIndex :type Integer))
  ;[1 1 1] Input
  (`self.DisableInput` (`GameplayStatics.GetPlayerController` 0))
  ;[1 1 1] Open door
  (`self.Close`)
  (goto _label_2 :!via `Reverse`))

(fn `SetKeyPress`
  (params (Input :type Boolean))
  (set `self.KeyPress` Input))

(fn `UserConstructionScript`)